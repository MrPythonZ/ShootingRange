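; BP_Ammo is a pickup that gives ammo to the first-person character when it overlaps the static mesh.
; Unless the pickup is already hiding, it adds AmmoAdded through a valid PlayerStatistics reference and plays a reload sound at its location.
; It then calls HidingForSomeTime, whose body is not shown here, which by name hides the pickup temporarily.
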(event OnComponentBeginOverlap(StaticMesh)
  (params (OverlappedComponent :type Primitive%20Component%20Object%20Reference) (OtherActor :type Actor%20Object%20Reference) (OtherComp :type Primitive%20Component%20Object%20Reference) (OtherBodyIndex :type Integer) (bFromSweep :type Boolean) (SweepResult :type Hit%20Result%20Structure%20%28by%20ref%29))
  (Class|KismetSystemLibrary|IsObjectOfSoftClass OtherActor "/Game/FirstPerson/Blueprints/BP_FirstPersonCharacter.BP_FirstPersonCharacter_C"
    (:True
      ;[1 1 1] Check if the actor is hiding
      (if (not (Variables|Default|GetInHiding))
        ;[1 1 1] Get the component reference for handling ammunitions
        (bind _playerstatistics (Variables|Default|GetPlayerStatistics)
          (:then
            ;[1 1 1] Add the ammo
            (Default|AddAmmo _playerstatistics (Variables|Default|GetAmmo%20Added))
            (Audio|PlaySoundatLocation "/Game/Sounds/S_Reload.S_Reload" (Transformation|GetWorldLocation (Variables|Default|GetDefaultSceneRoot)) "0, 0, 0" 1.0 1.0 0.0 0 0 0 0)
            (CallFunction|HidingforSomeTime))
          (:else))))))

(fn ConstructionScript)