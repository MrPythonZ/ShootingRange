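; BP_InteractableObject is an interactable actor that can hide itself in game for a set time.
; On BeginPlay it caches the AC_Statistic component from the player pawn as PlayerStatistics, though no logic here uses it.
; HidingForSomeTime toggles the hidden state and, when hiding, sets a timer of TimeHiding length to make the actor visible again.
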(event EventBeginPlay
  (Variables|Default|SetPlayerStatistics (Actor|GetComponentbyClass (Game|Player|GetPlayerPawn 0) "/Game/Blueprint/AC_Statistic.AC_Statistic_C")))

(fn ConstructionScript)

(fn HidingforSomeTime
  (Variables|Default|SetInHiding (not (Variables|Default|GetInHiding)))
  (Rendering|SetActorHiddenInGame self (Variables|Default|GetInHiding))
  (if (Variables|Default|GetInHiding)
    ;[0.15 0.15 0.15 0.5] If the actor is hiding, set a timer to make it visible again
    (Utilities|Time|SetTimerbyEvent (EventDispatchers|CreateEvent :!event HidingforSomeTime) (Variables|Default|GetTimeHiding))
    (return)
    (else
      (return))))