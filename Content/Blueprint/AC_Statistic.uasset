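; Actor component that tracks the player's score, ammo and hit combo, broadcasting change events for each.
; IncrementCombo adds score times the multiplier, raises it and starts a ResetCombo timer whose window shrinks with each hit.
; Score and ammo gains also accumulate in running totals sent with the events, with 2.5-second timers set on every gain.
; Helpers spend and check ammo and report the combo time remaining as a fraction.
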(fn AddStatistics
  (params (ScoreAdded :type Integer) (AmmoAdded :type Integer))
  ;[1 1 1] Updating score and ammo
  (UpdateStatistics|AddScore ScoreAdded)
  (UpdateStatistics|AddAmmo AmmoAdded)
  (return))

(fn PrintStatistics
  (Development|PrintString (Utilities|String|Append "Munizioni = " (Utilities|String|ToString(Integer) (Variables|Default|GetAmmo))) true true "(R=0.000000,G=0.660000,B=1.000000,A=1.000000)" 5e+01 "Ammo")
  (Development|PrintString (Utilities|String|Append "Punteggio = " (Utilities|String|ToString(Integer) (Variables|Default|GetScore))) true true "(R=0.000000,G=0.660000,B=1.000000,A=1.000000)" 5e+01 "Score"))

(fn ResetCombo
  (Variables|Default|SetCombo 1)
  (Variables|Default|SetTimerResetCombo (Variables|Default|GetMaxTimerReset))
  (Default|CallComboResetted)
  (return))

(fn IncrementCombo
  (params (ScoreIn :type Integer))
  (bind _returnvalue (Utilities|Time|SetTimerbyFunctionName 0 "ResetCombo" (Variables|Default|GetTimerResetCombo)))
  (Variables|Default|SetComboTimer _returnvalue)
  (UpdateStatistics|AddScore (* ScoreIn (Variables|Default|GetCombo)))
  (Math|Integer|IncrementInt (Variables|Default|GetCombo)
    (:%20%20
      ;[0.15 0.15 0.15 0.5] The combo expires sooner based on the number of targets hit
      (Variables|Default|SetTimerResetCombo (- (Variables|Default|GetTimerResetCombo) 0.2))
      (Default|CallComboChanged (Variables|Default|GetCombo))
      (return))))

(fn AddScore
  (params (Adding%20Score :type Integer))
  (if (> Adding%20Score 0)
    (bind _output_get (Variables|Default|SetScore (+ Adding%20Score (Variables|Default|GetScore))))
    (bind _result (UpdateStatistics|UpdateTotScoreAdded Adding%20Score))
    (Default|CallScoreChanged _result _output_get)
    (return)))

(fn UpdateTotScoreAdded
  (params (Value :type Integer))
  (bind _output_get (Variables|Default|SetTotScoreAdded (+ (Variables|Default|GetTotScoreAdded) Value)))
  (Utilities|Time|SetTimerbyEvent (EventDispatchers|CreateEvent :!event ResetTotScoreAdded) 2.5)
  (return _output_get))

(fn ResetTotScoreAdded
  (Variables|Default|SetTotScoreAdded 0))

(fn AddAmmo
  (params (Adding%20Ammo :type Integer))
  (if (> Adding%20Ammo 0)
    (bind _output_get (Variables|Default|SetAmmo (+ Adding%20Ammo (Variables|Default|GetAmmo))))
    (bind _result (UpdateStatistics|UpdateTotAmmoAdded Adding%20Ammo))
    (Default|CallAmmoChanged _result _output_get)
    (return)))

(fn UpdateTotAmmoAdded
  (params (Value :type Integer))
  (bind _output_get (Variables|Default|SetTotAmmoAdded (+ Value (Variables|Default|GetTotAmmoAdded))))
  (Utilities|Time|SetTimerbyEvent (EventDispatchers|CreateEvent :!event ResetAmmoAdded) 2.5)
  (return _output_get))

(fn ResetAmmoAdded
  (Variables|Default|SetTotAmmoAdded 0)
  (return))

(fn UseAmmo
  (bind _result (Math|Integer|DecrementInt (Variables|Default|GetAmmo))
    (:%20%20
      (return _result))))

(fn GetComboTimeRemainingPercent
  (return (/ (Utilities|Time|GetTimerRemainingTimebyHandle (Variables|Default|GetComboTimer)) (Variables|Default|GetTimerResetCombo))))

(fn TheresAmmo
  (return (> (Variables|Default|GetAmmo) 0)))